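; BP_QuestNpcComponent is an interaction component that lets a quest NPC open dialogue with the player.
; On Interact, it validates the interaction, calls the parent, then passes the NPC name, quest ID, quest-take flag and level's BP_QuestManager to BP_HUD's dialogue interface.
; FinishInteract calls the parent and switches the HUD back to the player view.
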(event `self.Interact`
  (bind _returnvalue (`self.CheckInteractionValid`))
  (if _returnvalue
    (`parent.Interact`)
    (bind _returnvalue_2 (`GameplayStatics.GetActorOfClass` "/Game/Blueprints/Quests/BP_QuestManager.BP_QuestManager_C"))
    (bind _asbp_hud (cast `/Game/Blueprints/UI/BP_HUD` (`PlayerController.GetHUD` (`GameplayStatics.GetPlayerController` 0))))
    (`/Game/Blueprints/UI/BP_HUD.ActiveDialogueInterface` _asbp_hud (`self.QuestNpcName`) (`self.QuestIDGive`) (`self.IsQuestTake`) _returnvalue_2)))

(event `self.FinishInteract`
  (`parent.FinishInteract`)
  (bind _asbp_hud (cast `/Game/Blueprints/UI/BP_HUD` (`PlayerController.GetHUD` (`GameplayStatics.GetPlayerController` 0))))
  (`/Game/Blueprints/UI/BP_HUD.ActiveHUDPlayer` _asbp_hud))